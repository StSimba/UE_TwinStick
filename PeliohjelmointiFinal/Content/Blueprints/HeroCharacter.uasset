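; Player hero character for a twin-stick shooter, with world-axis movement, stick aiming, a gun and respawn on death.
; Both look axes share one branch that turns the controller and pulls the gun trigger past a deadzone, releasing it otherwise.
; BeginPlay spawns the gun at the TempGun placeholder and stores the spawn transform in TwinStickMode.
; AffectHealth recalculates and prints health, then on death requests a respawn and destroys hero and gun.
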(event EventBeginPlay
  (bind _tempgun (Variables|Default|GetTempGun))
  (Utilities|FlowControl|Sequence
    (:then_0
      (bind _returnvalue (Game|SpawnActorfromClass "/Game/Blueprints/Gun.Gun_C" (Transformation|GetWorldTransform _tempgun) "Undefined" "MultiplyWithRoot" 0 0))
      (bind _output_get (Variables|Default|SetGun _returnvalue))
      (Transformation|AttachComponentToComponent _output_get _tempgun "None" "KeepWorld" "KeepWorld" "KeepWorld" true))
    (:then_1
      (bind _astwin_stick_mode (Utilities|Casting|CastToTwinStickMode (Game|GetGameMode)))
      (bind _output_get_2 (Variables|Default|SetGameMode _astwin_stick_mode))
      (Variables|/Game/Blueprints/TwinStickMode.TwinStickMode_C|SetPlayerSpawnTransform _output_get_2 (Transformation|GetActorTransform)))))

(event Collision|EventActorBeginOverlap
  (params (OtherActor :type Actor%20Object%20Reference)))

(event EventTick
  (params (DeltaSeconds :type Float%20%28single-precision%29)))

(event EventAffectHealth
  (params (Delta :type Float%20%28double-precision%29))
  (Class|BaseCharacter|HealthCalc Delta)
  (Development|PrintString (Utilities|String|ToString(Float) (Variables|Default|GetHealth)))
  (if (Variables|Default|GetisDead)
    (Default|RespawnPlayer (Variables|Default|GetGameMode))
    (Actor|DestroyActor self)))

(event Input|AxisEvents|InputAxisMoveUp
  (params (AxisValue :type Float%20%28single-precision%29))
  ;[0.15 0.15 0.15 0.5] Movement
  (Pawn|Input|AddMovementInput "1.000000,0.000000,0.000000" AxisValue false))

(event Input|AxisEvents|InputAxisMoveRight
  (params (AxisValue :type Float%20%28single-precision%29))
  ;[0.15 0.15 0.15 0.5] Movement
  (Pawn|Input|AddMovementInput "0.000000,1.000000,0.000000" AxisValue false))

(event Input|AxisEvents|InputAxisLookUp
  (params (AxisValue :type Float%20%28single-precision%29))
  (bind _gun (Variables|Default|GetGun))
  ;[0.15 0.15 0.15 0.5] Rotation
  (if (> (Math|Vector|VectorLength (Math|Vector|MakeVector AxisValue (stale Input|AxisEvents|InputAxisLookRight AxisValue) 0.0)) 0.25)
    (Pawn|SetControlRotation (Pawn|GetController) (Math|Conversions|RotationFromXVector (Math|Vector|MakeVector AxisValue (stale Input|AxisEvents|InputAxisLookRight AxisValue) 0.0)))
    (Default|PullTrigger _gun)
    (else
      (Default|ReleaseTrigger _gun))))

(event Input|AxisEvents|InputAxisLookRight
  (params (AxisValue :type Float%20%28single-precision%29))
  (bind _gun (Variables|Default|GetGun))
  ;[0.15 0.15 0.15 0.5] Rotation
  (if (> (Math|Vector|VectorLength (Math|Vector|MakeVector (stale Input|AxisEvents|InputAxisLookUp AxisValue) AxisValue 0.0)) 0.25)
    (Pawn|SetControlRotation (Pawn|GetController) (Math|Conversions|RotationFromXVector (Math|Vector|MakeVector (stale Input|AxisEvents|InputAxisLookUp AxisValue) AxisValue 0.0)))
    (Default|PullTrigger _gun)
    (else
      (Default|ReleaseTrigger _gun))))

(fn ConstructionScript)