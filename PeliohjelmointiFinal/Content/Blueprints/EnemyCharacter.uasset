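; Enemy character for a twin-stick game that damages the hero on overlap and awards score when killed.
; A looping timer applies damage while the hero overlaps and is cleared when that overlap ends.
; AffectHealth runs HealthCalc and, on death, ignores pawn and world-dynamic collision, increments the TwinStickMode score, detaches the controller and destroys the body after a delay.
; The construction script tints the body through a dynamic material instance.
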(event Custom|DamageToHero
  ;[0.15 0.15 0.15 0.5] Damage to player
  (Default|AffectHealth (Variables|Default|GetHero) (Variables|Default|GetDamage)))

(event EventBeginPlay)

(event Collision|EventActorBeginOverlap
  (params (OtherActor :type Actor%20Object%20Reference))
  ;[0.15 0.15 0.15 0.5] Begin damaging player on overlap
  (bind _ashero_character (Utilities|Casting|CastToHeroCharacter OtherActor))
  (Variables|Default|SetHero _ashero_character)
  (Utilities|Time|SetTimerbyFunctionName 0 "DamageToHero" 0.5 true true))

(event EventTick
  (params (DeltaSeconds :type Float%20%28single-precision%29)))

(event EventAffectHealth
  (params (Delta :type Float%20%28double-precision%29))
  (bind _capsulecomponent (Variables|Default|GetCapsuleComponent))
  ;[0.15 0.15 0.15 0.5] Health calculations and death check
  (Class|BaseCharacter|HealthCalc Delta)
  (if (Variables|Default|GetisDead)
    ;[0.15 0.15 0.15 0.5] When dead disable the enemy collision to player and bullets
    (Collision|SetCollisionResponsetoChannel _capsulecomponent "ECC_WorldDynamic" "ECR_Ignore")
    (Collision|SetCollisionResponsetoChannel _capsulecomponent "ECC_Pawn" "ECR_Ignore")
    ;[0.15 0.15 0.15 0.5] Added scoring system that adds score when enemy is killed
    (bind _astwin_stick_mode (Utilities|Casting|CastToTwinStickMode (Game|GetGameMode)))
    (Default|IncrementScore _astwin_stick_mode (Variables|Default|GetEnemyValue))
    ;[0.15 0.15 0.15 0.5] Removing the enemy's ability to move after death
    (Class|Pawn|DetachfromControllerPendingDestroy)
    ;[0.15 0.15 0.15 0.5] Destroy enemy body
    (Utilities|FlowControl|Delay 3.0)
    (Actor|DestroyActor)))

(event Collision|EventActorEndOverlap
  (params (OtherActor :type Actor%20Object%20Reference))
  ;[0.15 0.15 0.15 0.5] Check to end overlap
  (if (== OtherActor (Variables|Default|GetHero))
    (Utilities|Time|ClearTimerbyFunctionName 0 "DamageToHero")))

(fn ConstructionScript
  (bind _returnvalue (Rendering|Material|CreateDynamicMaterialInstance (Variables|Character|GetMesh) 0 0 "None" :!class /Script/Engine.PrimitiveComponent))
  (bind _output_get (Variables|Default|SetEnemyColor _returnvalue))
  (Rendering|Material|SetVectorParameterValue (Variables|Default|GetEnemyColor) "BodyColor" (Variables|Default|GetValue) :!class /Script/Engine.MaterialInstanceDynamic))